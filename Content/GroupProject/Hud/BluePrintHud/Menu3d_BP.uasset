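; Menu3d_BP is an actor for one screen of a 3D menu, hosting a 3dMenu_Widget and moving the player's view between linked menus.
; On BeginPlay it binds to the widget's transition event and disables its own collision.
; A transition index selects an entry from LinkMenus, then collision switches from this menu to the target while the view target blends to it with easing.
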(event `self.ReceiveBeginPlay`
  (bind _as3d_menu_widget (cast `/Game/GroupProject/Hud/INgameHud/3dMenu_Widget` (`WidgetComponent.GetUserWidgetObject` (`self.Widget`))))
  (add `/Game/GroupProject/Hud/INgameHud/3dMenu_Widget.Transition` _as3d_menu_widget (delegate `Ontransition`))
  (`self.SetActorEnableCollision` false))

(event `Ontransition`
  (params (MenuIndex :type Integer))
  (if (`KismetArrayLibrary.Array_IsValidIndex` (`self.LinkMenus`) MenuIndex)
    (`self.transitionTo` (`|GetArrayItem` (`self.LinkMenus`) MenuIndex))))

(event `transitionTo`
  (params (newMenu :type "/Game/GroupProject/Hud/BluePrintHud/Menu3d_BP Object Reference"))
  (`self.SetActorEnableCollision` false)
  (`self.SetActorEnableCollision` newMenu true)
  (`PlayerController.SetViewTargetWithBlend` (`GameplayStatics.GetPlayerController` 0) newMenu 2.0 "VTBlend_EaseInOut" 2.0 false))

(fn `UserConstructionScript`)