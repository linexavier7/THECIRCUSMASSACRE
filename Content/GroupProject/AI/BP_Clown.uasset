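; BP_Clown is an AI clown that moves toward the player and has logic for playing a laughing sound.
; On BeginPlay it issues a single AI MoveTo at player 0, stopping the laughing timeline on success.
; TryLaugh spawns the laugh sound at the clown when a downward capsule-radius sphere trace on Visibility hits.
; Its only caller is a timeline track that never runs, so the laugh does not play from this graph.
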(event `self.ReceiveBeginPlay`
  (`self.FollowPlayer`))

(event `FollowPlayer`
  (`|AIMoveTo` self (0.0 0.0 0.0) (`GameplayStatics.GetPlayerCharacter` 0)
    (:`OnSuccess`
      (`TimelineComponent.Stop` (`self.TL_Laughing`)))))

(fn `TraceLaughing`
  (returns (ReturnValue :type Boolean))
  (bind _returnvalue (`self.K2_GetActorLocation`))
  (bind _capsulecomponent (`self.CapsuleComponent`))
  (bind (_outhits _returnvalue_2) (`KismetSystemLibrary.SphereTraceMulti` _returnvalue (`KismetMathLibrary.MakeVector` (.x _returnvalue) (.y _returnvalue) (- (.z _returnvalue) (`CapsuleComponent.GetScaledCapsuleHalfHeight` _capsulecomponent))) (`CapsuleComponent.GetScaledCapsuleRadius` _capsulecomponent) "TraceTypeQuery1"))
  (return _returnvalue_2))

(fn `TryLaugh`
  (bind _returnvalue (`self.TraceLaughing`))
  (if _returnvalue
    (`GameplayStatics.SpawnSoundAtLocation` "/Game/GroupProject/Character/Clown/SFX/Laugh/ClownLaughing.ClownLaughing" (`self.K2_GetActorLocation`) (struct) 1.0 1.0 0.0 null null)))

(fn `UserConstructionScript`)