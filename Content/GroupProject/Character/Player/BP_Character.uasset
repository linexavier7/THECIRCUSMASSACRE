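; Player character with look and move input, running, a flashlight, inventory toggle, overlap-based interaction through Interact_BP, and a pause menu.
; Movement input plays or stops a footstep timeline by velocity, and running raises its play rate and walk speed.
; A downward sphere trace gates the footstep sound, but the timeline track calling it sits in never-run code.
; AnyDamage overwrites Heath with the damage value; its game-over branch is empty.
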(event `self.ReceiveBeginPlay`
  (bind _returnvalue (`|CreateWidget` "/Game/GroupProject/Hud/INgameHud/Pause_menu.Pause_menu_C"))
  (set `self.Ref_pause` _returnvalue))

(event `InputAction|PauseBTN` :paused true
  (params (Key :type "Key Structure"))
  (:`Pressed`
    (`/Engine/EditorBlueprintResources/StandardMacros.FlipFlop`
      (:`A`
        (set `PlayerController.bShowMouseCursor` true (`GameplayStatics.GetPlayerController` 0))
        (`GameplayStatics.SetGamePaused` true)
        (`UserWidget.AddToViewport` (`self.Ref_pause`) 0))
      (:`B`
        (set `PlayerController.bShowMouseCursor` false (`GameplayStatics.GetPlayerController` 0))
        (`GameplayStatics.SetGamePaused` false)
        (`Widget.RemoveFromParent` (`self.Ref_pause`))))))

(event `InputAxis|Turn`
  (params (AxisValue :type "Float (single-precision)"))
  ;[0 1 0.9791] Character Movements + Camera
  ;;[1 0 0] Camera
  (`self.AddControllerYawInput` AxisValue))

(event `InputAction|Run`
  (params (Key :type "Key Structure"))
  (bind _charactermovement (`self.CharacterMovement`))
  (bind _tl_footsteps (`self.TL_Footsteps`))
  ;[0 1 0.9791] Character Movements + Camera
  ;;[0.1683 0 0] Running
  (:`Pressed`
    (`TimelineComponent.SetPlayRate` _tl_footsteps 1.7)
    (set `CharacterMovementComponent.MaxWalkSpeed` 500.0 _charactermovement))
  (:`Released`
    (`TimelineComponent.SetPlayRate` _tl_footsteps 1.0)
    (set `CharacterMovementComponent.MaxWalkSpeed` 250.0 _charactermovement)))

(event `InputAxis|MoveForward`
  (params (AxisValue :type "Float (single-precision)"))
  (bind _tl_footsteps (`self.TL_Footsteps`))
  ;[0 1 0.9791] Character Movements + Camera
  ;;[0.4072 0 0] Movement
  (`self.AddMovementInput` (`SceneComponent.GetForwardVector` (`self.CapsuleComponent`)) AxisValue)
  (if (> (`KismetMathLibrary.VSize` (`self.GetVelocity`)) 0.0) :!label _label
    (`TimelineComponent.Play` _tl_footsteps)
    (else
      (`TimelineComponent.Stop` _tl_footsteps))))

(event `HaveFlashLight`
  (bind _spotlight (`self.SpotLight`))
  (bind _returnvalue (`SceneComponent.K2_GetComponentLocation` _spotlight))
  ;[1 1 1] FlashLight
  (if (`self.b_flashlight?`)
    (`SceneComponent.SetVisibility` _spotlight true false)
    (`GameplayStatics.PlaySoundAtLocation` "/Game/GroupProject/Sounds/Lanterna/FlashLight.FlashLight" _returnvalue (struct) 1.0 1.0 0.0 null null null null)
    (set `self.b_flashlight?` false)
    (else
      (`SceneComponent.SetVisibility` _spotlight false false)
      (`GameplayStatics.PlaySoundAtLocation` "/Game/GroupProject/Sounds/Lanterna/FlashLight.FlashLight" _returnvalue (struct) 1.0 1.0 0.0 null null null null)
      (set `self.b_flashlight?` true))))

(event `InputAxis|LookUp`
  (params (AxisValue :type "Float (single-precision)"))
  ;[0 1 0.9791] Character Movements + Camera
  ;;[1 0 0] Camera
  (`self.AddControllerPitchInput` AxisValue))

(event `InputAxis|MoveRight`
  (params (AxisValue :type "Float (single-precision)"))
  ;[0 1 0.9791] Character Movements + Camera
  ;;[0.4072 0 0] Movement
  (`self.AddMovementInput` (`SceneComponent.GetRightVector` (`self.CapsuleComponent`)) AxisValue)
  (goto _label))

(event `InputAction|FlashlightBTN`
  (params (Key :type "Key Structure"))
  ;[1 1 1] Lanterna No inventario
  (:`Pressed`
    (if (`self.haveFlashLight?`)
      (`self.HaveFlashLight`)
      (else
        (`KismetSystemLibrary.PrintString` "NãoTem lanterna")))))

(event `self.ReceiveTick`
  (params (DeltaSeconds :type "Float (single-precision)"))
  ;[0 0.3613 0.3564] Camera ON
)

(event `InputAction|InventarioBTN`
  (params (Key :type "Key Structure"))
  (:`Pressed`
    (`/Game/GroupProject/Inventario/Inventario_Component.toggleInvent` (`self.Inventario_Component`))))

(event `InputAction|InteractBTN`
  (params (Key :type "Key Structure"))
  ;[1 0.6031 0.6031] Interact
  (:`Pressed`
    (for _array_element (`self.GetOverlappingActors` "/Script/Engine.Actor")
      (if (`KismetSystemLibrary.DoesImplementInterface` _array_element "/Game/GroupProject/Inventario/Interact_BP.Interact_BP_C")
        (`GameplayStatics.PlaySoundAtLocation` "/Game/GroupProject/Sounds/Bag/bag.bag" (`SceneComponent.K2_GetComponentLocation` (`self.SpotLight`)) (struct) 1.0 1.0 0.0 null null null null)
        (message `/Game/GroupProject/Inventario/Interact_BP.Interact` _array_element self)
        (break)))))

(event `self.ReceiveAnyDamage`
  (params (Damage :type "Float (single-precision)") (DamageType :type "DamageType Object Reference") (InstigatedBy :type "Controller Object Reference") (DamageCauser :type "Actor Object Reference"))
  ;[1 1 1] Colocar a tela de gameover
  (set `self.Heath` Damage)
  (if (<= (`self.Heath`) 0.0)
    _))

(fn `TraceFootsteps`
  (returns (Finished :type Boolean))
  (bind _returnvalue (`self.K2_GetActorLocation`))
  (bind _capsulecomponent (`self.CapsuleComponent`))
  (bind (_outhit _returnvalue_2) (`KismetSystemLibrary.SphereTraceSingle` _returnvalue (`KismetMathLibrary.MakeVector` (.x _returnvalue) (.y _returnvalue) (- (.z _returnvalue) (`CapsuleComponent.GetScaledCapsuleHalfHeight` _capsulecomponent))) (`CapsuleComponent.GetScaledCapsuleRadius` _capsulecomponent) "TraceTypeQuery1"))
  (return _returnvalue_2))

(fn `TryFootstep`
  (bind _finished (`self.TraceFootsteps`))
  (if _finished
    (`GameplayStatics.PlaySoundAtLocation` "/Game/GroupProject/Character/Player/SFX/Footsteps/TileFootsteeps.TileFootsteeps" (`self.K2_GetActorLocation`) (struct) 1.0 1.0 0.0 null null null null)))

(fn `UserConstructionScript`)