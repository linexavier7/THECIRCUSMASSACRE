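; Key-locked door actor that swings open when the player character enters its trigger box and closes when they leave.
; Box overlap events act only while Havekey is true and the other actor is a BP_Character.
; Separate timelines drive the door's relative yaw: one plays from start to open, the other reverses from end to close, so each swing restarts rather than continuing from the current angle.
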(event `self.Box.OnComponentBeginOverlap`
  (params (OverlappedComponent :type "PrimitiveComponent Object Reference") (OtherActor :type "Actor Object Reference") (OtherComp :type "PrimitiveComponent Object Reference") (OtherBodyIndex :type Integer) (bFromSweep :type Boolean) (SweepResult :type "HitResult Structure (by ref)"))
  (if (`self.Havekey?`)
    (cast `/Game/GroupProject/Character/Player/BP_Character` OtherActor)
    (bind (_direction _opendoor) (`Timeline|OpenDoor` :!via `PlayFromStart`)
      (:`Update`
        (`SceneComponent.K2_SetRelativeRotation` (`self.door`) (`KismetMathLibrary.MakeRotator` 0.0 0.0 _opendoor) false false)))))

(event `self.Box.OnComponentEndOverlap`
  (params (OverlappedComponent :type "PrimitiveComponent Object Reference") (OtherActor :type "Actor Object Reference") (OtherComp :type "PrimitiveComponent Object Reference") (OtherBodyIndex :type Integer))
  (if (`self.Havekey?`)
    (cast `/Game/GroupProject/Character/Player/BP_Character` OtherActor)
    (bind (_direction _opendoor) (`Timeline|Timeline` :!via `ReverseFromEnd`)
      (:`Update`
        (`SceneComponent.K2_SetRelativeRotation` (`self.door`) (`KismetMathLibrary.MakeRotator` 0.0 0.0 _opendoor) false false)))))

(fn `UserConstructionScript`)